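; BP_Blade is a blade weapon actor that the player can pick up and equip in first person.
; PickUp detaches and destroys any blade in BP_Player's EquipBlade, stores itself there, and snaps onto the BladePoint socket of FirstPersonMesh.
; SwitchBlade is rudimentary, always setting the mesh to the first Blades entry.
; Debug prints remain, along with disconnected spawn and reposition nodes.
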(event EventSwitchBlade
  ;[1 1 1] Switching
  (Development|PrintString "Hello")
  (bind _output_get (Variables|Default|SetCurrentBlade (Utilities|Array|Get(acopy) (Variables|Default|GetBlades))))
  (Components|StaticMesh|SetStaticMesh (Variables|Default|GetBlade) _output_get))

(event EventPickUp
  (bind _returnvalue (Game|GetPlayerCharacter 0))
  (bind _asbp_player (Utilities|Casting|CastToBP_Player _returnvalue))
  ;[1 1 1] Pick Up
  (Utilities|IsValid (Variables|/Game/FirstPerson/Blueprints/BP_Player.BP_Player_C|GetEquipBlade (.AsBP%20Player (Utilities|Casting|CastToBP_Player (Game|GetPlayerCharacter 0))))
    (:Is%20Valid
      (Transformation|DetachFromActor (Variables|/Game/FirstPerson/Blueprints/BP_Player.BP_Player_C|GetEquipBlade (.AsBP%20Player (Utilities|Casting|CastToBP_Player (Game|GetPlayerCharacter 0)))) "KeepRelative" "KeepRelative" "KeepRelative")
      (Actor|DestroyActor (Variables|/Game/FirstPerson/Blueprints/BP_Player.BP_Player_C|GetEquipBlade (.AsBP%20Player (Utilities|Casting|CastToBP_Player (Game|GetPlayerCharacter 0))))))
    (:Is%20Not%20Valid
      _))
  (bind _output_get (Variables|/Game/FirstPerson/Blueprints/BP_Player.BP_Player_C|SetEquipBlade _asbp_player self))
  (Development|PrintString (Utilities|GetDisplayName _output_get))
  (Transformation|AttachComponentToComponent (Variables|/Game/FirstPerson/Blueprints/BP_Player.BP_Player_C|GetFirstPersonMesh _asbp_player) "BladePoint" "SnapToTarget" "SnapToTarget" "SnapToTarget" true))

(fn ConstructionScript)