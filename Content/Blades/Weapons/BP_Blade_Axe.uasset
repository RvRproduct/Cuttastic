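; Axe blade weapon that the player picks up, switches to and slashes with to cut enemies.
; Pickup and switch events attach the equipped blade to the first-person mesh socket, with pickup also adding it to the inventory.
; While slashing, Tick runs HitDetect, a counter-gated sphere trace along blade sockets.
; Matching CutType slices the enemy's procedural mesh horizontally or vertically, launches the cut half, and destroys the enemy after a delay.
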(event EventSwitchBlade
  (bind _returnvalue (Game|GetPlayerCharacter 0))
  (bind _asbp_player (Utilities|Casting|CastToBP_Player _returnvalue))
  ;[1 1 1] Switching
  (Utilities|IsValid (Variables|/Game/FirstPerson/Blueprints/BP_Player.BP_Player_C|GetEquipBlade _asbp_player)
    (:Is%20Valid
      (Transformation|DetachFromActor (Variables|/Game/FirstPerson/Blueprints/BP_Player.BP_Player_C|GetEquipBlade _asbp_player) "KeepRelative" "KeepRelative" "KeepRelative")
      (bind _output_get (Variables|/Game/FirstPerson/Blueprints/BP_Player.BP_Player_C|SetEquipBlade _asbp_player (Variables|/Game/FirstPerson/Blueprints/BP_Player.BP_Player_C|GetChangeBlade (.AsBP%20Player (Utilities|Casting|CastToBP_Player (Game|GetPlayerCharacter 0))))))
      (Development|PrintString (Utilities|GetDisplayName _output_get))
      (Transformation|AttachComponentToComponent _output_get (Variables|/Game/FirstPerson/Blueprints/BP_Player.BP_Player_C|GetFirstPersonMesh _asbp_player) "BladePoint_Axe" "SnapToTarget" "SnapToTarget" "SnapToTarget" true))))

(event EventTick
  (params (DeltaSeconds :type Float%20%28single-precision%29))
  ;[1 1 1] Hit Detection
  (if (Variables|/Game/FirstPerson/Blueprints/BP_Player.BP_Player_C|GetSlashing (.AsBP%20Player (Utilities|Casting|CastToBP_Player (Game|GetPlayerCharacter 0))))
    (bind (_enemy _hitenemy) (CallFunction|HitDetect))
    (Utilities|FlowControl|Delay 1e+01)
    (if _hitenemy
      (Actor|DestroyActor _enemy))))

(event EventPickUp
  (bind _returnvalue (Game|GetPlayerCharacter 0))
  (bind _asbp_player (Utilities|Casting|CastToBP_Player _returnvalue))
  ;[1 1 1] Pick Up
  (Utilities|IsValid (Variables|/Game/FirstPerson/Blueprints/BP_Player.BP_Player_C|GetEquipBlade (.AsBP%20Player (Utilities|Casting|CastToBP_Player (Game|GetPlayerCharacter 0))))
    (:Is%20Valid
      (Transformation|DetachFromActor (Variables|/Game/FirstPerson/Blueprints/BP_Player.BP_Player_C|GetEquipBlade (.AsBP%20Player (Utilities|Casting|CastToBP_Player (Game|GetPlayerCharacter 0)))) "KeepRelative" "KeepRelative" "KeepRelative"))
    (:Is%20Not%20Valid
      _))
  (bind _output_get (Variables|/Game/FirstPerson/Blueprints/BP_Player.BP_Player_C|SetEquipBlade _asbp_player self))
  (Transformation|AttachComponentToComponent (Variables|/Game/FirstPerson/Blueprints/BP_Player.BP_Player_C|GetFirstPersonMesh _asbp_player) "BladePoint_Axe" "SnapToTarget" "SnapToTarget" "SnapToTarget" true)
  ;[1 1 1] Adding To Inventory
  (Utilities|Array|Add (Variables|/Game/FirstPerson/Blueprints/BP_Player.BP_Player_C|GetInventory (.AsBP%20Player (Utilities|Casting|CastToBP_Player (Game|GetPlayerCharacter 0)))) _output_get))

(fn ConstructionScript)

(fn HitDetect
  (bind _blade (Variables|Default|GetBlade))
  (bind _output_get (Variables|Default|SetSlashTimer (+ (Variables|Default|GetSlashTimer) 1)))
  (Math|Integer|CompareInt _output_get 60
    (:>
      (bind (_outhit _returnvalue) (Collision|SphereTraceForObjects (Transformation|GetSocketLocation _blade "Start") (Transformation|GetSocketLocation _blade "End") 2e+01 (Utilities|Array|MakeArray "ObjectTypeQuery1") false 0 "Persistent"))
      (bind _asbp_enemy (Utilities|Casting|CastToBP_Enemy (.HitActor (Collision|BreakHitResult _outhit))))
      (Variables|/Game/Enemy/BP_Enemy.BP_Enemy_C|SetAlive _asbp_enemy (not (Utilities|Enum|Equal(Enum) (Variables|/Game/Enemy/BP_Enemy.BP_Enemy_C|GetCutType _asbp_enemy) (Variables|Default|GetCutType))))
      (if (Utilities|Enum|Equal(Enum) (Variables|/Game/Enemy/BP_Enemy.BP_Enemy_C|GetCutType _asbp_enemy) (Variables|Default|GetCutType))
        (bind _asprocedural_mesh_component (Utilities|Casting|CastToProceduralMeshComponent (.HitComponent (Collision|BreakHitResult _outhit))))
        (Actor|GetAllActorsOfClass "/Game/FirstPerson/Blueprints/BP_Cutting/BP_FirstPersonCharacter_testSylvia.BP_FirstPersonCharacter_testSylvia_C")
        (bind _asbp_player (Utilities|Casting|CastToBP_Player (Game|GetPlayerCharacter 0)))
        (if (Variables|/Game/FirstPerson/Blueprints/BP_Player.BP_Player_C|GetHorizontalSlash _asbp_player)
          (Variables|Default|SetPlane%20Normal "0.000000,0.000000,1.000000")
          (else
            (Variables|Default|SetPlane%20Normal "0.000000,1.000000,0.000000")))
        (Development|PrintString (Utilities|String|ToString(Vector) (Variables|Default|GetPlane%20Normal)))
        (bind _outotherhalfprocmesh (Class|KismetProceduralMeshLibrary|SliceProceduralMesh _asprocedural_mesh_component (.ImpactPoint (Collision|BreakHitResult _outhit)) (Variables|Default|GetPlane%20Normal) true "CreateNewSectionForCap" "/Game/FPWeapon/Materials/BaseMaterial.BaseMaterial"))
        (Physics|SetSimulatePhysics _outotherhalfprocmesh true)
        (Physics|AddImpulse _outotherhalfprocmesh "300.000000,300.000000,300.000000" "None" true)
        (Variables|Default|SetSlashTimer 0)
        (return _asbp_enemy _returnvalue)
        (else
          (Development|PrintString "Type not equa"))))))