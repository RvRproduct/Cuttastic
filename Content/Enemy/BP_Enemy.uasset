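; Enemy that detects, chases and shoots the player, using a procedural mesh copied from its Cube static mesh.
; While alive, Tick acquires a target component through a forward sphere trace or nearby overlap, falling back to an empty Patrol stub.
; A tracked target is dropped at long range, approached at mid range, or faced and shot at up close.
; Shooting spawns first-person projectiles ahead of the mesh, throttled by a call counter against CoolDown.
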(event EventBeginPlay)

(event Collision|EventActorBeginOverlap
  (params (OtherActor :type Actor%20Object%20Reference)))

(event EventTick
  (params (DeltaSeconds :type Float%20%28single-precision%29))
  (if (Variables|Default|GetAlive)
    (if (Variables|Components|GetTracking)
      (Math|Float|CompareFloat (Math|Vector|Distance(Vector) (Transformation|GetWorldLocation (Variables|Default|GetProceduralMesh)) (Transformation|GetWorldLocation (Variables|Default|GetTrackedPlayer))) 4e+03
        (:>
          (Variables|Components|SetTracking false)
          (Development|PrintString "Lose track"))
        (:==
          (Math|Float|CompareFloat (Math|Vector|Distance(Vector) (Transformation|GetWorldLocation (Variables|Default|GetProceduralMesh)) (Transformation|GetWorldLocation (Variables|Default|GetTrackedPlayer))) 2e+03 :!label _label
            (:>
              (CallFunction|MoveTowardPlayer (Variables|Default|GetTrackedPlayer) :!label _label_2)
              (Development|PrintString "Move"))
            (:==
              (goto _label_2))
            (:<
              (CallFunction|ShootatPlayer (Variables|Default|GetTrackedPlayer) (Variables|Default|Getcount))
              (Development|PrintString "Shoot"))))
        (:<
          (goto _label)))
      (else
        (bind (_ifhit _player) (CallFunction|Track))
        (if _ifhit
          (Variables|Default|SetTrackedPlayer _player)
          (Variables|Components|SetTracking true)
          (else
            (CallFunction|Patrol)))))))

(fn ConstructionScript
  (Class|KismetProceduralMeshLibrary|CopyProceduralMeshfromStaticMeshComponent (Variables|Default|Getcube) 0 (Variables|Default|GetProceduralMesh) true)
  (Variables|Default|SetCutType "NewEnumerator0"))

(fn MoveTowardPlayer
  (params (Player :type Primitive%20Component%20Object%20Reference))
  (bind _returnvalue (Transformation|GetWorldLocation Player))
  (bind _proceduralmesh (Variables|Default|GetProceduralMesh))
  (bind _returnvalue_2 (Transformation|GetWorldLocation _proceduralmesh))
  (Class|MovementComponent|MoveUpdatedComponent (Variables|Components|GetFloatingPawnMovement) (Math|Vector|Normalize (- _returnvalue _returnvalue_2)) (Math|Rotator|FindLookatRotation _returnvalue_2 _returnvalue) true))

(fn Track
  (bind _proceduralmesh (Variables|Default|GetProceduralMesh))
  (bind _returnvalue (Transformation|GetWorldLocation _proceduralmesh))
  (bind (_outhit _returnvalue_2) (Collision|SphereTraceForObjects _returnvalue (+ _returnvalue (* (Math|Vector|GetForwardVector (Transformation|GetWorldRotation _proceduralmesh)) 2e+03)) 5e+02 (Variables|Components|GetObject%20Types_0) false 0 "ForOneFrame"))
  (if _returnvalue_2
    (return true (.HitComponent (Collision|BreakHitResult _outhit)))
    (else
      (bind (_outcomponents _returnvalue_3) (Collision|SphereOverlapComponents (Transformation|GetWorldLocation (Variables|Default|GetProceduralMesh)) 1e+03 (LocalVariables|Getcharacater%20type)))
      (if _returnvalue_3
        (Development|PrintString "Hello")
        (return true (Utilities|Array|Get(acopy) _outcomponents))
        (else
          (return false 0))))))

(fn ShootatPlayer
  (params (Player :type Primitive%20Component%20Object%20Reference) (count :type Integer))
  (bind _proceduralmesh (Variables|Default|GetProceduralMesh))
  (bind _returnvalue (Transformation|GetWorldRotation _proceduralmesh))
  (bind _output_get (Variables|Default|Setcount (+ 1 count)))
  (Transformation|SetWorldRotation (Variables|Default|GetProceduralMesh) (Math|Rotator|FindLookatRotation (Transformation|GetWorldLocation (Variables|Default|GetProceduralMesh)) (Transformation|GetWorldLocation Player)) false false)
  (Math|Integer|CompareInt _output_get (LocalVariables|GetCoolDown)
    (:>
      (Game|SpawnActorfromClass "/Game/FirstPerson/Blueprints/BP_FirstPersonProjectile.BP_FirstPersonProjectile_C" (Math|Transform|MakeTransform (+ (Transformation|GetWorldLocation _proceduralmesh) (Math|Vector|RotateVector "300.000000,0.000000,0.000000" _returnvalue)) _returnvalue) "Undefined" "OverrideRootScale" 0 0)
      (Variables|Default|Setcount 0))))

(fn Patrol)